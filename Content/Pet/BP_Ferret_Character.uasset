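; Ferret pet character that wanders at random and stops to face the player when spoken to.
; From BeginPlay, WalkToRandom loops AI moves to random reachable points nearby, pausing between attempts and only waiting while Standing is set.
; BeginSpeaking sets Standing, halts the AI and turns the capsule's yaw toward the player through a timeline.
; EndSpeaking clears Standing so wandering resumes; the delay after the turn triggers nothing.
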(event Custom|WalkToRandom
  (if (Variables|Default|GetStanding)
    _
    (else
      (AI|AIMoveTo (AI|GetAIController self) (.RandomLocation (AI|Navigation|GetRandomReachablePointinRadius (Transformation|GetWorldLocation (Variables|Collision|GetCapsuleComponent)) 8e+02 0 0)) 0 -1.0 "Default" "Default" true true
        (:OnRequestFailed
          _)
        (:OnMoveFinished
          _))))
  (Utilities|FlowControl|Delay 4.0)
  (CallFunction|WalktoRandom))

(event Custom|BeginSpeaking
  (bind _capsulecomponent (Variables|Collision|GetCapsuleComponent))
  (Variables|Default|SetStanding true)
  (AI|Navigation|StopMovement (AI|GetAIController self))
  (bind _turnamount (Timeline|RotateToPlayer PlayFromStart)
    (:Update
      (Transformation|SetWorldRotation (Variables|Collision|GetCapsuleComponent) (Math|Rotator|MakeRotator 0.0 0.0 (Math|Float|Lerp (.yaw (Transformation|GetWorldRotation _capsulecomponent)) (.yaw (Math|Rotator|FindLookatRotation (Transformation|GetWorldLocation _capsulecomponent) (Transformation|GetActorLocation (Game|Player|GetPlayerPawn 0)))) _turnamount)) false false))
    (:Finished
      (Utilities|FlowControl|Delay 12.0))))

(event Custom|EndSpeaking
  (Variables|Default|SetStanding false))

(event EventBeginPlay
  (CallFunction|WalktoRandom))

(event Collision|EventActorBeginOverlap
  (params (OtherActor :type Actor%20Object%20Reference)))

(event EventTick
  (params (DeltaSeconds :type Float%20%28single-precision%29)))

(fn ConstructionScript)